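; Input handler for the Cameroid camera that takes over the controls from the player while the camera is in use.
; Use switches input from the player to this Blueprint; the Cameroid action unequips the camera and hands input back.
; While active, it handles look with the player's sensitivity and invert settings, takes photos on Use and toggles the flash on Alternative Use.
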(event `self.ReceiveBeginPlay`
  (bind _asmaster (`/Game/HorrorEngine/Blueprints/Core/HE_Functions.GetPlayer`))
  (set `self.Player` _asmaster))

(event `self.Use`
  (params (HorrorEvent :type Boolean))
  (`/Game/HorrorEngine/Blueprints/Core/HE_Functions.PlayerInput` false)
  (`self.ControllerInput` true))

(event `EnhancedInput|/Game/HorrorEngine/Input/HE_AlternativeUse`
  (params (ActionValue :type Boolean) (ElapsedSeconds :type "Float (double-precision)") (TriggeredSeconds :type "Float (double-precision)") (InputAction :type "InputAction Object Reference" :default "/Game/HorrorEngine/Input/HE_AlternativeUse.HE_AlternativeUse"))
  (bind _player (`self.Player`))
  (:`Started`
    (set `/Game/HorrorEngine/Blueprints/Player/HorrorEngine.CameroidFlashOn` (not (`/Game/HorrorEngine/Blueprints/Player/HorrorEngine.CameroidFlashOn` _player)) _player)))

(event `EnhancedInput|/Game/HorrorEngine/Input/HE_Look`
  (params (ActionValue :type "Vector2D Structure") (ElapsedSeconds :type "Float (double-precision)") (TriggeredSeconds :type "Float (double-precision)") (InputAction :type "InputAction Object Reference" :default "/Game/HorrorEngine/Input/HE_Look.HE_Look"))
  (bind _returnvalue (`GameplayStatics.GetPlayerCharacter` 0))
  (bind _player (`self.Player`))
  (bind _camerasensivity (`/Game/HorrorEngine/Blueprints/Player/HorrorEngine.CameraSensivity` _player))
  (:`Triggered`
    (`Pawn.AddControllerYawInput` _returnvalue (* ActionValue_X (select `bool` (`/Game/HorrorEngine/Blueprints/Player/HorrorEngine.InvertCameraH` _player) :`false` 1.0 :`true` -1.0) _camerasensivity))
    (`Pawn.AddControllerPitchInput` _returnvalue (* ActionValue_Y (select `bool` (`/Game/HorrorEngine/Blueprints/Player/HorrorEngine.InvertCameraV` _player) :`false` 1.0 :`true` -1.0) _camerasensivity))))

(event `EnhancedInput|/Game/HorrorEngine/Input/HE_Use`
  (params (ActionValue :type Boolean) (ElapsedSeconds :type "Float (double-precision)") (TriggeredSeconds :type "Float (double-precision)") (InputAction :type "InputAction Object Reference" :default "/Game/HorrorEngine/Input/HE_Use.HE_Use"))
  (:`Started`
    (`/Game/HorrorEngine/Blueprints/Player/HorrorEngine.TakePhoto` (`self.Player`))))

(event `EnhancedInput|/Game/HorrorEngine/Input/HE_Cameroid`
  (params (ActionValue :type Boolean) (ElapsedSeconds :type "Float (double-precision)") (TriggeredSeconds :type "Float (double-precision)") (InputAction :type "InputAction Object Reference" :default "/Game/HorrorEngine/Input/HE_Cameroid.HE_Cameroid"))
  (:`Started`
    (`/Game/HorrorEngine/Blueprints/Player/HorrorEngine.UnequipCameroid` (`self.Player`))
    (`self.ControllerInput` false)
    (`/Game/HorrorEngine/Blueprints/Core/HE_Functions.PlayerInput` true)))

(fn `UserConstructionScript`)