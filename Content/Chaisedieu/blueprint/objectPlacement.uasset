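; Puzzle placement zone that feeds a number to a code manager when the matching object is placed in it.
; On begin overlap, an actor tagged with ObjetName adds NumCode to CodeManager, and ending that overlap removes it.
; The AlreadyAdd flag prevents the number from being added twice, and debug prints in English and French report overlaps, additions, wrong tags and removals.
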(event `self.ReceiveActorBeginOverlap`
  (params (OtherActor :type "Actor Object Reference"))
  (`KismetSystemLibrary.PrintString` "Overlap")
  (if (`self.AlreadyAdd`)
    _
    (elif (`self.ActorHasTag` OtherActor (`self.ObjetName`))
      (set `self.AlreadyAdd` true)
      (`/Game/Blueprints/codeManager.AddNumber` (`self.CodeManager`) (`self.NumCode`))
      (`KismetSystemLibrary.PrintString` "Numéro ajouté")
      (else
        (`KismetSystemLibrary.PrintString` "Mauvais tag")))))

(event `self.ReceiveActorEndOverlap`
  (params (OtherActor :type "Actor Object Reference"))
  (if (`self.AlreadyAdd`)
    (if (`self.ActorHasTag` OtherActor (`self.ObjetName`))
      (`/Game/Blueprints/codeManager.RemoveNumber` (`self.CodeManager`) (`self.NumCode`))
      (set `self.AlreadyAdd` false)
      (`KismetSystemLibrary.PrintString` "Numéro enlevé"))))

(fn `UserConstructionScript`)