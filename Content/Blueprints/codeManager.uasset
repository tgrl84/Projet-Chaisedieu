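; Code manager for a four-digit puzzle that activates a linked actor when the correct sequence is entered.
; AddNumber collects digits and, at four, checks that each equals its array index, so the solution is 0-1-2-3 in order.
; A match prints a success message and calls Use on the Actor; a mismatch clears the code, prints a failure message and resets every referenced cube.
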(event `AddNumber`
  (params (num :type Integer))
  (bind _code (`self.code`))
  (`KismetArrayLibrary.Array_Add` _code num)
  (if (== (`KismetArrayLibrary.Array_Length` _code) 4)
    (for (_array_element _array_index) (`self.code`)
      (if (== _array_element _array_index)
        (set `self.isCodeCorrect` true)
        (else
          (`KismetArrayLibrary.Array_Clear` (`self.code`))
          (set `self.isCodeCorrect` false)
          (break))))
    (if (`self.isCodeCorrect`)
      (`KismetSystemLibrary.PrintString` "Code bon")
      (`/Game/HorrorEngine/Blueprints/Core/Use.Use` (`self.Actor`) false)
      (else
        (`KismetSystemLibrary.PrintString` "code mauvais")
        (for _array_element_2 (`self.cubes`)
          (`/Game/Chaisedieu/torchCode.Reset` _array_element_2))))))

(fn `UserConstructionScript`)